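; BP_GameMaster drives the day cycle by rotating a directional light in step with game time.
; On BeginPlay it waits briefly for the save to load, then pitches the light to match the game instance's elapsed time, at 15 degrees per game hour.
; A looping timer then adds a quarter-degree of pitch every game minute, with hour length taken from BP_GossipGameMode.
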(event Custom|Advance
  (Transformation|AddActorLocalRotation (Variables|Default|GetDirectionalLight) (Math|Rotator|MakeRotator 0.0 (Math|Float|MakeLiteralFloat 0.25) 0.0) false false))

(event EventBeginPlay
  (bind _returnvalue (Game|GetGameMode))
  (bind _asbp_gossip_game_mode (Utilities|Casting|CastToBP_GossipGameMode _returnvalue))
  (bind _gamehourdurationseconds (Variables|/Script/Gossip.GossipGameMode|GetGameHourDurationSeconds _asbp_gossip_game_mode))
  (bind _returnvalue_2 (/ _gamehourdurationseconds 6e+01))
  (Utilities|FlowControl|Delay 0.2) ; Ensure LoadGame is Done
  (Transformation|AddActorLocalRotation (Variables|Default|GetDirectionalLight) (Math|Rotator|MakeRotator 0.0 (* (/ (Variables|/Script/Gossip.GS_GameInstance|GetRealGameTimeSeconds (.AsGS%20Game%20Instance (Utilities|Casting|CastToGS_GameInstance (Game|GetGameInstance)))) _gamehourdurationseconds) 15.0) 0.0) false false)
  (Utilities|Time|SetTimerbyEvent (delegate Custom|Advance) _returnvalue_2 true _returnvalue_2))

(fn ConstructionScript)