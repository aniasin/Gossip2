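; BP_Npc is an AI-controlled NPC with an instincts component and a bubble widget that displays its current AI state.
; The construction script copies instinct info from the component's data asset when the component's own list is empty.
; Every tick, it casts to GS_AIController and writes the current action and goal enum names, concatenated without a separator, into the BP_Bubble text block.
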(event EventTick
  (params (DeltaSeconds :type Float%20%28single-precision%29))
  (bind _returnvalue (Pawn|GetController))
  (bind _asgs_aicontroller (Utilities|Casting|CastToGS_AIController _returnvalue))
  (Rendering|Components|TextRender|SetText (Variables|/Game/UI/BP_Bubble.BP_Bubble_C|GetTextBlock_221 (.AsBP%20Bubble (Utilities|Casting|CastToBP_Bubble (UserInterface|GetWidget (Variables|Default|GetWidget))))) (Utilities|Text|ToText(String) (Utilities|String|Append (Utilities|String|EnumtoString (Variables|/Script/Gossip.GS_AIController|GetCurrentAction _asgs_aicontroller)) " 
" (Utilities|String|EnumtoString (Variables|/Script/Gossip.GS_AIController|GetCurrentGoal _asgs_aicontroller))))))

(fn ConstructionScript
  (bind _instinctscomp (Variables|Default|GetInstinctsComp))
  (if (<= (Utilities|Array|Length (Variables|/Script/Gossip.InstinctsComponent|GetInstinctsInfo _instinctscomp)) 0)
    (Variables|/Script/Gossip.InstinctsComponent|SetInstinctsInfo _instinctscomp (Variables|/Script/Gossip.InstinctsDataAsset|GetInstinctsInfo (Variables|/Script/Gossip.InstinctsComponent|GetInstinctDataAsset _instinctscomp)))))