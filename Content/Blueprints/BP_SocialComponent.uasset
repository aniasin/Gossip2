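; BP_SocialComponent is a component that shows a dialog widget on screen above its owning actor.
; Its Dialog event creates a BP_Dialog for the first player controller, initializes it with the given Proximity value and plays it.
; The widget is placed once, by projecting a point at a fixed height above the owner's location to screen space, so this graph does not update its position afterward.
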(event EventDialog
  (params (Proximity :type Integer))
  (bind _returnvalue (Components|GetOwner))
  (bind _returnvalue_2 (Transformation|GetActorLocation _returnvalue))
  (bind _returnvalue_3 (UserInterface|CreateWidget "/Game/MenuSystem/UI/BP_Dialog.BP_Dialog_C" (Game|GetPlayerController 0)))
  (Default|Initialize _returnvalue_3 Proximity)
  (Class|UserWidget|SetPositioninViewport _returnvalue_3 (.ScreenPosition (Class|GameplayStatics|ProjectWorldtoScreen (Game|GetPlayerController 0) (Math|Vector|MakeVector (.x _returnvalue_2) (.y _returnvalue_2) (+ (.z _returnvalue_2) 1.6e+02)) false)) true)
  (UserInterface|Viewport|AddtoViewport _returnvalue_3 0)
  (Default|Play _returnvalue_3))