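; BP_Shelter is a shelter item actor that carries persistent identifiers for itself and a spawned NPC.
; Its construction script generates SpawnedNpcId and OwnId once, only when each is still invalid, so existing values survive reconstruction.
; A newly generated OwnId is also copied into the SaveComponent as its Id.
; The event graph holds only disabled default events, so no runtime logic lives in this Blueprint's graphs.
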(event EventBeginPlay)

(event Collision|EventActorBeginOverlap
  (params (OtherActor :type Actor%20Object%20Reference)))

(event EventTick
  (params (DeltaSeconds :type Float%20%28single-precision%29)))

(fn ConstructionScript
  (Utilities|FlowControl|Sequence
    (:then_0
      (if (not (Guid|IsValidGuid (Variables|Default|GetSpawnedNpcId)))
        (Variables|Default|SetSpawnedNpcId (Guid|NewGuid))))
    (:then_1
      (if (not (Guid|IsValidGuid (Variables|Default|GetOwnId)))
        (bind _output_get (Variables|Default|SetOwnId (Guid|NewGuid)))
        (Variables|/Script/Gossip.SaveableEntity|SetId (Variables|Default|GetSaveComponent) _output_get)))))