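; BP_RessourceCollector is a resource item Blueprint whose mesh follows its resource type and whose color reflects resource state.
; The construction script finds the matching RessourceType in RessourceData, synchronously loads its soft mesh reference, then creates a dynamic instance of MI_Solid.
; The material's "Base Color" starts as LivingColor, is reapplied on BeginPlay, and changes to the color passed by RessourceStateChanged.
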(event EventBeginPlay
  (Rendering|Material|SetVectorParameterValue (Variables|Default|GetDynamicMaterialRef) "Base Color" (Variables|Default|GetLivingColor) :!class /Script/Engine.MaterialInstanceDynamic))

(event EventRessourceStateChanged
  (params (Color :type Linear%20Color%20Structure))
  (Rendering|Material|SetVectorParameterValue (Variables|Default|GetDynamicMaterialRef) "Base Color" Color :!class /Script/Engine.MaterialInstanceDynamic))

(fn ConstructionScript
  (bind _mesh (Variables|Character|GetMesh))
  (Utilities|FlowControl|Sequence
    (:then_0
      (bind _array_element (Utilities|Array|ForEachLoopwithBreak (Variables|/Script/Gossip.RessourceDataAsset|GetRessourceDataArray (Variables|Default|GetRessourceData)) :!label _label)
        (:LoopBody
          (if (Utilities|Enum|Equal(Enum) (Variables|Default|GetRessourceType) (.RessourceType (Utilities|Struct|BreakRessourceData _array_element)))
            (bind _returnvalue (Utilities|LoadAssetBlocking (.MeshSoftObject (Utilities|Struct|BreakRessourceData _array_element))))
            (Components|StaticMesh|SetStaticMesh (Variables|Character|GetMesh) (.AsStatic%20Mesh (Utilities|Casting|CastToStaticMesh _returnvalue)))
            (goto _label Break)))))
    (:then_1
      (Rendering|Material|SetMaterial _mesh 0 "/Game/LevelPrototyping/Materials/MI_Solid.MI_Solid")
      (bind _returnvalue_2 (Rendering|Material|CreateDynamicMaterialInstance _mesh 0 (Rendering|Material|GetMaterial _mesh 0) "None" :!class /Script/Engine.PrimitiveComponent))
      (bind _output_get (Variables|Default|SetDynamicMaterialRef _returnvalue_2))
      (Rendering|Material|SetVectorParameterValue _output_get "Base Color" (Variables|Default|GetLivingColor) :!class /Script/Engine.MaterialInstanceDynamic))))