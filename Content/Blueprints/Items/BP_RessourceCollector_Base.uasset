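; Base Blueprint for a resource collector item whose mesh and collection settings depend on its resource type.
; Its construction script looks up the entry matching RessourceType in the RessourceData list, then applies that entry's mesh and copies its Raw and WaitTime values.
; The event graph holds only unused default events, so the file itself contains no collection logic.
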(event EventBeginPlay)

(event Collision|EventActorBeginOverlap
  (params (OtherActor :type Actor%20Object%20Reference)))

(event EventTick
  (params (DeltaSeconds :type Float%20%28single-precision%29)))

(fn ConstructionScript
  (bind _array_element (Utilities|Array|ForEachLoopwithBreak (Variables|/Script/Gossip.RessourceDataAsset|GetRessourceData (Variables|Default|GetRessourceData)) :!label _label)
    (:LoopBody
      (if (Utilities|Enum|Equal(Enum) (Variables|Default|GetRessourceType) (.RessourceType (Utilities|Struct|BreakRessourceData _array_element)))
        (Components|StaticMesh|SetStaticMesh (Variables|Default|GetStaticMesh) (.Mesh (Utilities|Struct|BreakRessourceData _array_element)))
        (Variables|Default|SetbRaw (.bRaw (Utilities|Struct|BreakRessourceData _array_element)))
        (Variables|Default|SetWaitTime (.WaitTime (Utilities|Struct|BreakRessourceData _array_element)))
        (goto _label Break)))))